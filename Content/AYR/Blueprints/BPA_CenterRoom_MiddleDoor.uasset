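; Construction-time builder for the walls of a center room, assembled from instanced mesh tiles on the Room component.
; The construction script calls CreateRoom, which stacks eleven rows downward on a 200-unit grid.
; Each row lays two pairs of opposite walls sized by Length and Width, rotating and nudging tiles per side.
; Despite the MiddleDoor name, the graphs contain no door logic or runtime behavior.
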(event EventBeginPlay)

(fn ConstructionScript
  (CallFunction|CreateRoom))

(fn CreateRoom
  (for _index (range 0 10)
    (LocalVariables|SetHighWallOffset (* _index 2e+02))
    (for _index_2 (range 0 1)
      (Utilities|FlowControl|Sequence
        (:then_0
          (for _index_3 (range 0 (- (Variables|Default|GetLength) 3))
            (Components|InstancedStaticMesh|AddInstance (Variables|Default|GetRoom) (Math|Transform|MakeTransform (Math|Vector|MakeVector (.X (Math|Vector|BreakVector (+ (+ (Math|Vector|MakeVector (+ (* _index_2 (* (- (Variables|Default|GetWidth) 2) -2e+02)) -1e+02) (* _index_3 2e+02) -1.1e+02) "-100.000000,200.000000,0.000000") (* "-20.000000, 0, 0" _index_2)))) (.Y (Math|Vector|BreakVector (+ (+ (Math|Vector|MakeVector (+ (* _index_2 (* (- (Variables|Default|GetWidth) 2) -2e+02)) -1e+02) (* _index_3 2e+02) -1.1e+02) "-100.000000,200.000000,0.000000") (* "-20.000000, 0, 0" _index_2)))) (+ (* -1 (LocalVariables|GetHighWallOffset)) -2e+02)) (Math|Rotator|MakeRotator 0.0 9e+01 (* _index_2 1.8e+02)) "1.000001,1.000001,1.000001"))))
        (:then_1
          (for _index_4 (range 0 (- (Variables|Default|GetWidth) 3))
            (Components|InstancedStaticMesh|AddInstance (Variables|Default|GetRoom) (Math|Transform|MakeTransform (Math|Vector|MakeVector (.X (Math|Vector|BreakVector (+ (+ (Math|Vector|MakeVector (* _index_4 -2e+02) (* _index_2 (* (- (Variables|Default|GetLength) 2) 2e+02)) -1.1e+02) "-310.000000,90.000000,-100.000000") (* "0.000000,20.000000, 0" _index_2)))) (.Y (Math|Vector|BreakVector (+ (+ (Math|Vector|MakeVector (* _index_4 -2e+02) (* _index_2 (* (- (Variables|Default|GetLength) 2) 2e+02)) -1.1e+02) "-310.000000,90.000000,-100.000000") (* "0.000000,20.000000, 0" _index_2)))) (+ (* -1 (LocalVariables|GetHighWallOffset)) -2e+02)) (Math|Rotator|MakeRotator 9e+01 0.0 (* _index_2 1.8e+02)) "1.000001,1.000001,1.000001"))))))))