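; Delivery machine actor that dispenses an ID card when it receives a configurable gameplay message.
; A general state machine moves it from idling to opening when that message arrives.
; On opening, it plays the machine animation, spawns an ID card of the configured type and attaches it to a socket.
; Destroying the card broadcasts the room-change message to hide the floor.
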(event Custom|OpenDeliver
  (params (Message :type GMS%20Message%20Base%20Object%20Reference))
  (Class|GeneralStateMachineComponent|ChangeStateto (Variables|Default|GetGeneralStateMachine) (Variables|Default|GetOpeningStateName)))

(event Custom|OnIDCardDestroyed
  (params (DestroyedActor :type Actor%20Object%20Reference))
  (Class|GameplayMessageSubsystem|Broadcast (Subsystems|GetGameplayMessageSubsystem) "(TagName=\"GMSMessage.Gameplay.ChangeRoom.HideFloor\")"))

(event Custom|OnIdlingStateChangeToOpeningState
  (Audio|Components|Audio|Play (Variables|Default|GetDeliverMachine) false)
  (bind _returnvalue (Game|SpawnActorfromClass "/Game/AYR/Blueprints/Interactable/IDCard/BPA_IDCard.BPA_IDCard_C" (Math|Transform|MakeTransform "0, 0, 0" "0, 0, 0" "1,1,1") "Undefined" 0 (Variables|Default|GetIDCard%20Type) 0))
  (bind _output_get (Variables|Default|SetIDCard _returnvalue))
  (Transformation|AttachComponentToComponent _output_get (Variables|Default|GetDeliverMachine) "IDCardLocation" "KeepRelative" "KeepRelative" "KeepWorld" true)
  (Game|BindEventtoOnDestroyed (Variables|Default|GetIDCard) (EventDispatchers|CreateEvent :!event Custom|OnIDCardDestroyed)))

(event EventBeginPlay
  (bind _generalstatemachine (Variables|Default|GetGeneralStateMachine))
  (bind _returnvalue (Class|GameplayMessageSubsystem|Register (Subsystems|GetGameplayMessageSubsystem) (Variables|Default|GetOpeningGMSTag) (EventDispatchers|CreateEvent :!event Custom|OpenDeliver)))
  (Variables|Default|SetGMSHandle _returnvalue)
  (Class|GeneralStateMachineComponent|CreateStateMachineNode _generalstatemachine (Variables|Default|GetIdlingStateName))
  (Class|GeneralStateMachineComponent|CreateStateMachineNode _generalstatemachine (Variables|Default|GetOpeningStateName))
  (Class|GeneralStateMachineComponent|SetStateMachineConditionwithAction _generalstatemachine (Variables|Default|GetIdlingStateName) (Variables|Default|GetOpeningStateName) (EventDispatchers|CreateEvent :!event Custom|OnIdlingStateChangeToOpeningState))
  (Class|GeneralStateMachineComponent|InitGeneralStateMachine (Variables|Default|GetGeneralStateMachine) (Variables|Default|GetIdlingStateName)))

(event EventEndPlay
  (params (EndPlayReason :type EEndPlayReason%20Enum :default "Destroyed"))
  (bind _gmshandle (Variables|Default|GetGMSHandle))
  (if (Class|GameplayMessageSubsystem|IsHandleValid _gmshandle)
    (Class|GameplayMessageSubsystem|Unregister (Subsystems|GetGameplayMessageSubsystem) _gmshandle)))

(fn ConstructionScript)