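; Kill volume that sends the game back to the MainMenu level when an actor overlaps it.
; Overlap starts a fade out with a callback for the level change, and records initial ACHV_Dead achievement progress if the cached value is still zero.
; It registers for a DisableKillVolume gameplay message to switch off its collision, and unregisters on EndPlay.
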(event Custom|FadeOut
  (Class|GameWorldSubsystem|OpenNewLevel (Subsystems|GetGameWorldSubsystem) "MainMenu"))

(event Custom|OnDisableMessageReceived
  (params (Message :type GMS%20Message%20Base%20Object%20Reference))
  (Collision|SetCollisionEnabled (Variables|Default|GetCollisionComponent) "NoCollision"))

(event EventBeginPlay
  (bind _returnvalue (Class|GameplayMessageSubsystem|Register (Subsystems|GetGameplayMessageSubsystem) "(TagName=\"GMSMessage.Gameplay.DisableKillVolume\")" (EventDispatchers|CreateEvent :!event Custom|OnDisableMessageReceived)))
  (Variables|Default|SetDisableKillVolumeGMSHandle _returnvalue))

(event EventEndPlay
  (params (EndPlayReason :type EEndPlayReason%20Enum :default "Destroyed"))
  (Class|GameplayMessageSubsystem|Unregister (Subsystems|GetGameplayMessageSubsystem) (Variables|Default|GetDisableKillVolumeGMSHandle)))

(event Collision|EventActorBeginOverlap
  (params (OtherActor :type Actor%20Object%20Reference))
  (bind _returnvalue (Game|GetPlayerController 0))
  (Class|GameWorldSubsystem|StartFadewithEvent (Subsystems|GetGameWorldSubsystem) (EventDispatchers|CreateEvent :!event Custom|FadeOut) "DefaultFadeOut")
  (bind (_bfoundid _progress) (Class|AchievementBlueprintLibrary|GetCachedAchievementProgress _returnvalue "ACHV_Dead"))
  (if (and _bfoundid (<= _progress 0.0))
    (|WriteAchievementProgress _returnvalue "ACHV_Dead" 0.1)))

(fn ConstructionScript)