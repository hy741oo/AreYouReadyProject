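; Main menu button actor that shows its enabled or disabled state through the emissive color of its static mesh.
; It starts disabled in red, and a Gameplay Message Subsystem EnableButton message turns it green and plays a 2D confirm sound.
; Color changes go through dynamic material instances, and the message listener is unregistered on EndPlay.
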(event Custom|EnableButton
  (bind _returnvalue (Rendering|Material|CreateDynamicMaterialInstance (Variables|Default|GetStaticMesh) 0 0 "None" :!class /Script/Engine.PrimitiveComponent))
  (Rendering|Material|SetVectorParameterValue _returnvalue "EmissiveColor" "(R=0.000000,G=1.000000,B=0.000000,A=1.000000)" :!class /Script/Engine.MaterialInstanceDynamic))

(event Custom|DisableButton
  (bind _returnvalue (Rendering|Material|CreateDynamicMaterialInstance (Variables|Default|GetStaticMesh) 0 0 "None" :!class /Script/Engine.PrimitiveComponent))
  (Rendering|Material|SetVectorParameterValue _returnvalue "EmissiveColor" "(R=1.000000,G=0.000000,B=0.000000,A=1.000000)" :!class /Script/Engine.MaterialInstanceDynamic))

(event Custom|OnMessageReceived
  (params (Message :type GMS%20Message%20Base%20Object%20Reference))
  (CallFunction|EnableButton)
  (Audio|PlaySound2D (Subsystems|GetAudioSubsystem) "MainLevel_InteractiveButtonConfirm" -1.0 self))

(event EventBeginPlay
  (CallFunction|DisableButton)
  (bind _returnvalue (Class|GameplayMessageSubsystem|Register (Subsystems|GetGameplayMessageSubsystem) "(TagName=\"GMSMessage.Gameplay.MainMenu.EnableButton\")" (EventDispatchers|CreateEvent :!event Custom|OnMessageReceived)))
  (Variables|Default|SetGMSHandle _returnvalue))

(event Collision|EventActorBeginOverlap
  (params (OtherActor :type Actor%20Object%20Reference)))

(event EventTick
  (params (DeltaSeconds :type Float%20%28single-precision%29)))

(event EventEndPlay
  (params (EndPlayReason :type EEndPlayReason%20Enum :default "Destroyed"))
  (bind _gmshandle (Variables|Default|GetGMSHandle))
  (if (Class|GameplayMessageSubsystem|IsHandleValid _gmshandle)
    (Class|GameplayMessageSubsystem|Unregister (Subsystems|GetGameplayMessageSubsystem) _gmshandle)))

(fn ConstructionScript)