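; Room actor that builds a walled room from instanced meshes, with a flickering ceiling light and sliding door.
; The construction script rebuilds floor, ceiling and walls from length, width and height, leaving a doorway gap.
; Gameplay messages drive the door timeline forward or backward and start the flicker timeline.
; Flicker triggers toggle light, audio and emissive material, then that listener unregisters when the timeline finishes.
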(event Custom|StartFlashLight
  (params (Message :type GMS%20Message%20Base%20Object%20Reference))
  (Timeline|FlashLight Play
    (:Finished
      (CallFunction|UnregisterFlashLightMessage))
    (:Trigger
      (Utilities|FlowControl|FlipFlop
        (:A
          (CallFunction|TurnOffLight))
        (:B
          (CallFunction|TurnonLight))))))

(event Custom|TurnOnLight
  (Rendering|SetVisibility (Variables|Default|GetRectLight) true false)
  (Components|Activation|Activate (Variables|Default|GetAudio) false)
  (Rendering|Material|SetScalarParameterValueonMaterials (Variables|Default|GetCeilingLightStaticMesh) "EmissiveScaler" 1.0))

(event Custom|TurnOffLight
  (Rendering|SetVisibility (Variables|Default|GetRectLight) false false)
  (Components|Activation|Deactivate (Variables|Default|GetAudio))
  (Rendering|Material|SetScalarParameterValueonMaterials (Variables|Default|GetCeilingLightStaticMesh) "EmissiveScaler" 0.0))

(event Custom|UnregisterFlashLightMessage
  (Class|GameplayMessageSubsystem|Unregister (Subsystems|GetGameplayMessageSubsystem) (Variables|GMSHandle|GetFlashLightGMSHandle)))

(event Custom|OpenDoor
  (bind _door (Variables|Default|GetDoor))
  (bind _relativelocation (Variables|/Script/Engine.SceneComponent|GetRelativeLocation _door))
  (bind (_x _y _z) (Math|Vector|BreakVector _relativelocation))
  (bind _doorrelativeylocation (Timeline|DoorMovementTimeline Play)
    (:Update
      (Transformation|SetRelativeLocation _door (Math|Vector|MakeVector _x _doorrelativeylocation _z) false false))))

(event Custom|CloseDoor
  (bind _door (Variables|Default|GetDoor))
  (bind _relativelocation (Variables|/Script/Engine.SceneComponent|GetRelativeLocation _door))
  (bind (_x _y _z) (Math|Vector|BreakVector _relativelocation))
  (bind _doorrelativeylocation (Timeline|DoorMovementTimeline Reverse)
    (:Update
      (Transformation|SetRelativeLocation _door (Math|Vector|MakeVector _x _doorrelativeylocation _z) false false))))

(event Custom|OnOpeningDoorMessageReceived
  (params (Message :type GMS%20Message%20Base%20Object%20Reference))
  (CallFunction|OpenDoor))

(event Custom|OnClosingDoorMessageReceived
  (params (Message :type GMS%20Message%20Base%20Object%20Reference))
  (CallFunction|CloseDoor))

(event EventBeginPlay
  (bind _returnvalue (Subsystems|GetGameplayMessageSubsystem))
  (bind _returnvalue_2 (Class|GameplayMessageSubsystem|Register _returnvalue "(TagName=\"GMSMessage.Gameplay.StartRoom.FlashLight\")" (EventDispatchers|CreateEvent :!event Custom|StartFlashLight)))
  (Variables|GMSHandle|SetFlashLightGMSHandle _returnvalue_2)
  (bind _returnvalue_3 (Class|GameplayMessageSubsystem|Register _returnvalue (Variables|GMSTag|GetOpeningDoorGMSTag) (EventDispatchers|CreateEvent :!event Custom|OnOpeningDoorMessageReceived)))
  (Variables|GMSHandle|SetOpeningDoorGMSHandle _returnvalue_3)
  (bind _returnvalue_4 (Class|GameplayMessageSubsystem|Register _returnvalue (Variables|GMSTag|GetClosingOpeningDoorGMSTag) (EventDispatchers|CreateEvent :!event Custom|OnClosingDoorMessageReceived)))
  (Variables|GMSHandle|SetClosingDoorGMSHandle _returnvalue_4))

(event EventEndPlay
  (params (EndPlayReason :type EEndPlayReason%20Enum :default "Destroyed"))
  (bind _returnvalue (Subsystems|GetGameplayMessageSubsystem))
  (CallFunction|UnregisterFlashLightMessage)
  (Class|GameplayMessageSubsystem|Unregister _returnvalue (Variables|GMSHandle|GetOpeningDoorGMSHandle))
  (Class|GameplayMessageSubsystem|Unregister _returnvalue (Variables|GMSHandle|GetClosingDoorGMSHandle)))

(fn ConstructionScript
  (Components|InstancedStaticMesh|ClearInstances (Variables|Default|GetRoom))
  (CallFunction|CreateRoom (Variables|Default|GetRoomLength) (Variables|Default|GetRoomWidth) (Variables|Default|GetRoomHeight)))

(fn CreateRoom
  (params (Length :type Integer) (Width :type Integer) (Height :type Integer))
  (Utilities|FlowControl|Sequence
    (:then_0
      (LocalVariables|SetLengthIndex (- Length 1))
      (LocalVariables|SetWidthIndex (- Width 1))
      (LocalVariables|SetHeightIndex (- Height 1)))
    (:then_1
      (for _index (range 0 1)
        ;[1 1 1] Z轴方向上的墙壁
        (for _index_2 (range 0 (LocalVariables|GetWidthIndex))
          (for _index_3 (range 0 (LocalVariables|GetLengthIndex))
            (Components|InstancedStaticMesh|AddInstance (Variables|Default|GetRoom) (Math|Transform|MakeTransform (Math|Vector|MakeVector (* _index_3 2e+02) (* _index_2 2e+02) (+ (* _index (* (Variables|Default|GetRoomHeight) 2e+02)) (* _index 2e+01))) (Math|Rotator|MakeRotator (* _index 1.8e+02) 0.0 0.0) "1,1,1"))))
        ;[1 1 1] Y轴方向上的墙壁
        (for _index_4 (range 0 (LocalVariables|GetHeightIndex))
          (for _index_5 (range 0 (LocalVariables|GetLengthIndex))
            (Components|InstancedStaticMesh|AddInstance (Variables|Default|GetRoom) (Math|Transform|MakeTransform (Math|Vector|MakeVector (* _index_5 2e+02) (+ (- (* _index (* (Variables|Default|GetRoomWidth) 2e+02)) 1.1e+02) (* _index 2e+01)) (+ (* _index_4 2e+02) 1.1e+02)) (Math|Rotator|MakeRotator (+ 9e+01 (* _index 1.8e+02)) 0.0 0.0) "1,1,1"))))
        ;[1 1 1] X轴方向的墙壁
        (for _index_6 (range 0 (LocalVariables|GetHeightIndex))
          (for _index_7 (range 0 (LocalVariables|GetWidthIndex))
            (if (Math|Boolean|ORBoolean (> _index_7 0) (> _index_6 1) (> _index 0))
              (Components|InstancedStaticMesh|AddInstance (Variables|Default|GetRoom) (Math|Transform|MakeTransform (Math|Vector|MakeVector (+ (- (* _index (* (Variables|Default|GetRoomLength) 2e+02)) 1.1e+02) (* _index 2e+01)) (* _index_7 2e+02) (+ (* _index_6 2e+02) 1.1e+02)) (Math|Rotator|MakeRotator 0.0 (+ -9e+01 (* _index 1.8e+02)) 0.0) "1,1,1")))))))))