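; BPA_StartRoom is the start room actor that runs a scripted flickering light effect with audio.
; It registers for the StartRoom FlashLight gameplay message on BeginPlay, and the listener plays the FlashLight timeline.
; Timeline trigger events drive a FlipFlop that toggles the RectLight's visibility and the audio component together.
; The listener unregisters when the timeline finishes, making the effect one-shot, or on EndPlay.
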(event Custom|StartFlashLight
  (params (Message :type GMS%20Message%20Base%20Object%20Reference))
  (Timeline|FlashLight Play
    (:Finished
      (CallFunction|UnregisterFlashLightMessage))
    (:Trigger
      (Utilities|FlowControl|FlipFlop
        (:A
          (CallFunction|TurnOffLight))
        (:B
          (CallFunction|TurnonLight))))))

(event Custom|TurnOnLight
  (Rendering|SetVisibility (Variables|Default|GetRectLight) true false)
  (Components|Activation|Activate (Variables|Default|GetAudio) false))

(event Custom|TurnOffLight
  (Rendering|SetVisibility (Variables|Default|GetRectLight) false false)
  (Components|Activation|Deactivate (Variables|Default|GetAudio)))

(event Custom|UnregisterFlashLightMessage
  (Class|GameplayMessageSubsystem|Unregister (Subsystems|GetGameplayMessageSubsystem) (Variables|Default|GetFlashLightGMSHandle)))

(event EventBeginPlay
  (bind _returnvalue (Class|GameplayMessageSubsystem|Register (Subsystems|GetGameplayMessageSubsystem) "(TagName=\"GMSMessage.Gameplay.StartRoom.FlashLight\")" (EventDispatchers|CreateEvent :!event Custom|StartFlashLight)))
  (Variables|Default|SetFlashLightGMSHandle _returnvalue))

(event EventEndPlay
  (params (EndPlayReason :type EEndPlayReason%20Enum :default "Destroyed"))
  (CallFunction|UnregisterFlashLightMessage))

(fn ConstructionScript)