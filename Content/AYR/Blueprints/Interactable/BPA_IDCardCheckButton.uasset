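; An interactable button Blueprint that gates its condition on the ID cards the player holds.
; It overrides CheckConditionInternal, casting player 0 to MainLevelCharacter and testing each Blue, Green or Red entry in the CheckType list against that character's card flags.
; Every listed card is required: the check fails on the first missing card or a failed cast, and an empty list passes.
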(fn ConstructionScript
  (|CallParentFunction))

(fn CheckConditionInternal
  (bind _asmain_level_character (Utilities|Casting|CastToMainLevelCharacter (Game|GetPlayerCharacter 0))
    (:then
      (for _array_element (Variables|Default|GetCheckType)
        (switch Utilities|FlowControl|Switch|SwitchonE_IDCardType _array_element
          (:NewEnumerator0
            (if (not (Class|MainLevelCharacter|HaveGotBlueIDCard _asmain_level_character))
              (return false)))
          (:NewEnumerator1
            (if (not (Class|MainLevelCharacter|HaveGotGreenIDCard _asmain_level_character))
              (return false)))
          (:NewEnumerator2
            (if (not (Class|MainLevelCharacter|HaveGotRedIDCard _asmain_level_character))
              (return false)))))
      (return true))
    (:CastFailed
      (return false))))