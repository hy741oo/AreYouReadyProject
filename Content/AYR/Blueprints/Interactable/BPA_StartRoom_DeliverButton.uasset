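; Interactable deliver button for the start room that gives color and sound feedback when used, then locks briefly before re-arming.
; BeginPlay builds a two-state machine (interactive and not interactive), with enter delegates that tint the mesh's emissive material green or red.
; Interact switches to not interactive, whose transition action plays a confirm sound, and returns to interactive after a short delay.
; No delivery logic lives in this graph.
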(event Custom|OnEnterNotInteractiveState
  (bind _returnvalue (Rendering|Material|CreateDynamicMaterialInstance (Variables|Default|GetStaticMesh) 0 0 "None" :!class /Script/Engine.PrimitiveComponent))
  (Rendering|Material|SetVectorParameterValue _returnvalue "EmissiveColor" "(R=1.000000,G=0.000000,B=0.000000,A=1.000000)" :!class /Script/Engine.MaterialInstanceDynamic))

(event Custom|OnEnterInteractiveState
  (bind _returnvalue (Rendering|Material|CreateDynamicMaterialInstance (Variables|Default|GetStaticMesh) 0 0 "None" :!class /Script/Engine.PrimitiveComponent))
  (Rendering|Material|SetVectorParameterValue _returnvalue "EmissiveColor" "(R=0.000000,G=1.000000,B=0.000000,A=1.000000)" :!class /Script/Engine.MaterialInstanceDynamic))

(event Custom|OnEnterNotInteractiveStateConditionPassed
  (CallFunction|PlayConfirmSound))

(event EventBeginPlay
  (bind _generalstatemachine (Variables|Default|GetGeneralStateMachine))
  (bind _interactivestatename (Variables|Default|GetInteractiveStateName))
  (bind _notinteractivestatename (Variables|Default|GetNotInteractiveStateName))
  (bind _generalstatemachine_2 (Variables|Default|GetGeneralStateMachine))
  (Utilities|FlowControl|Sequence
    (:then_0
      (Class|GeneralStateMachineComponent|CreateStateMachineNodeBP _generalstatemachine _interactivestatename)
      (Class|GeneralStateMachineComponent|SetStateMachineNodeonEnterStateDelegate _generalstatemachine _interactivestatename (EventDispatchers|CreateEvent :!event Custom|OnEnterInteractiveState))
      (Class|GeneralStateMachineComponent|SetStateMachineConditionwithAction _generalstatemachine _interactivestatename (Variables|Default|GetNotInteractiveStateName) (EventDispatchers|CreateEvent :!event Custom|OnEnterNotInteractiveStateConditionPassed)))
    (:then_1
      (Class|GeneralStateMachineComponent|CreateStateMachineNodeBP _generalstatemachine_2 _notinteractivestatename)
      (Class|GeneralStateMachineComponent|SetStateMachineNodeonEnterStateDelegate _generalstatemachine_2 _notinteractivestatename (EventDispatchers|CreateEvent :!event Custom|OnEnterNotInteractiveState))
      (Class|GeneralStateMachineComponent|SetStateMachineCondition _generalstatemachine_2 _notinteractivestatename (Variables|Default|GetInteractiveStateName)))
    (:then_2
      (Class|GeneralStateMachineComponent|InitGeneralStateMachine (Variables|Default|GetGeneralStateMachine) (Variables|Default|GetInteractiveStateName)))))

(event EventInteract
  (Class|GeneralStateMachineComponent|ChangeStateto (Variables|Default|GetGeneralStateMachine) (Variables|Default|GetNotInteractiveStateName))
  (Utilities|FlowControl|Delay 2.0)
  (Class|GeneralStateMachineComponent|ChangeStateto (Variables|Default|GetGeneralStateMachine) (Variables|Default|GetInteractiveStateName)))

(fn ConstructionScript)