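; Interactable escape button that ends the game when the player uses it and returns them to the main menu.
; Interact disables player input and starts the WorldManager's game-over fade with an end callback, presumably OnPlayerEscape.
; OnPlayerEscape opens MainMenu through the WorldManager, then writes progress to the escape achievement if its cached entry exists with no progress yet.
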(event Custom|OnPlayerEscape
  (bind _returnvalue (Game|GetPlayerController 0))
  (Class|WorldManager|OpenNewLevel (Subsystems|GetWorldManager) "MainMenu")
  (bind (_bfoundid _progress) (Class|AchievementBlueprintLibrary|GetCachedAchievementProgress _returnvalue "ACHV_Escape"))
  (if (and _bfoundid (<= _progress 0.0))
    (|WriteAchievementProgress _returnvalue "ACHV_Escape" 0.1)))

(event EventBeginPlay
  (|CallParentFunction) ; This node is disabled and will not be called.\nDrag off pins to build functionality.
)

(event Collision|EventActorBeginOverlap
  (params (OtherActor :type Actor%20Object%20Reference)))

(event EventTick
  (params (DeltaSeconds :type Float%20%28single-precision%29)))

(event EventInteract
  (|CallParentFunction)
  (Input|DisableInput (Game|GetPlayerController 0) 0)
  (Class|WorldManager|StartFadewithEvent (Subsystems|GetWorldManager) (EventDispatchers|CreateEvent :!event Custom|OnPlayerEscape) "GameOverFadeOut"))

(fn ConstructionScript
  (|CallParentFunction))