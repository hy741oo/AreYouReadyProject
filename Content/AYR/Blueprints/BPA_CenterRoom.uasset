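; Procedural center room actor that builds a tall rectangular room around a central pit, sized by Width and Length.
; The construction script runs CreateRoom, which adds rotated 200-unit tiles to one instanced mesh, Room.
; Outer walls stack upward with an opening at each corner in the bottom two layers, and inner walls mirror downward inside a one-tile floor ledge.
; The ledge sits inside the height loop, so its instances repeat on every layer.
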(event EventBeginPlay)

(fn ConstructionScript
  (CallFunction|CreateRoom))

(fn CreateRoom
  (bind _width (Variables|Default|GetWidth))
  (bind _length (Variables|Default|GetLength))
  (bind _returnvalue (- _length 1))
  (bind _returnvalue_2 (- _width 1))
  (for _index (range 0 10)
    (LocalVariables|SetHighWallOffset (* _index 2e+02))
    (for _index_2 (range 0 1)
      (Utilities|FlowControl|Sequence
        (:then_0
          (for _index_3 (range 0 _returnvalue)
            (if (Math|Boolean|ORBoolean (and (== _index_2 0) (> _index_3 0)) (>= _index 2) (and (== _index_2 1) (< _index_3 _returnvalue)))
              (Components|InstancedStaticMesh|AddInstance (Variables|Default|GetRoom) (Math|Transform|MakeTransform (Math|Vector|MakeVector (+ (* _index_2 -2e+01) (* _index_2 (* (Variables|Default|GetWidth) -2e+02))) (* _index_3 2e+02) (LocalVariables|GetHighWallOffset)) (Math|Rotator|MakeRotator 0.0 9e+01 (* _index_2 1.8e+02)) "1,1,1")))))
        (:then_1
          (for _index_4 (range 0 _returnvalue_2)
            (if (Math|Boolean|ORBoolean (and (== _index_2 1) (> _index_4 0)) (>= _index 2) (and (== _index_2 0) (< _index_4 _returnvalue_2)))
              (Components|InstancedStaticMesh|AddInstance (Variables|Default|GetRoom) (Math|Transform|MakeTransform (+ (Math|Vector|MakeVector (* _index_4 -2e+02) (+ (* _index_2 2e+01) (* _index_2 (* (Variables|Default|GetLength) 2e+02))) (LocalVariables|GetHighWallOffset)) "-110.000000,-110.000000, 0") (Math|Rotator|MakeRotator 9e+01 0.0 (* _index_2 1.8e+02)) "1,1,1")))))
        (:then_2
          (for _index_5 (range 0 (- (Variables|Default|GetLength) 1))
            (Components|InstancedStaticMesh|AddInstance (Variables|Default|GetRoom) (Math|Transform|MakeTransform (Math|Vector|MakeVector (+ (* _index_2 (* (- (Variables|Default|GetWidth) 1) -2e+02)) -1.1e+02) (* _index_5 2e+02) -1.1e+02) "0, 0, 0" "1,1,1"))))
        (:then_3
          (for _index_6 (range 0 (- (Variables|Default|GetWidth) 3))
            (Components|InstancedStaticMesh|AddInstance (Variables|Default|GetRoom) (Math|Transform|MakeTransform (+ (Math|Vector|MakeVector (* _index_6 -2e+02) (* _index_2 (* (- (Variables|Default|GetLength) 1) 2e+02)) -1.1e+02) "-310.000000, 0, 0") "0, 0, 0" "1,1,1"))))
        (:then_4
          (for _index_7 (range 0 (- (Variables|Default|GetLength) 3))
            (Components|InstancedStaticMesh|AddInstance (Variables|Default|GetRoom) (Math|Transform|MakeTransform (Math|Vector|MakeVector (.X (Math|Vector|BreakVector (+ (+ (Math|Vector|MakeVector (+ (* _index_2 (* (- (Variables|Default|GetWidth) 2) -2e+02)) -1e+02) (* _index_7 2e+02) -1.1e+02) "-100.000000,200.000000,0.000000") (* "-20.000000, 0, 0" _index_2)))) (.Y (Math|Vector|BreakVector (+ (+ (Math|Vector|MakeVector (+ (* _index_2 (* (- (Variables|Default|GetWidth) 2) -2e+02)) -1e+02) (* _index_7 2e+02) -1.1e+02) "-100.000000,200.000000,0.000000") (* "-20.000000, 0, 0" _index_2)))) (+ (* -1 (LocalVariables|GetHighWallOffset)) -2e+02)) (Math|Rotator|MakeRotator 0.0 9e+01 (* _index_2 1.8e+02)) "1,1,1"))))
        (:then_5
          (for _index_8 (range 0 (- (Variables|Default|GetWidth) 3))
            (Components|InstancedStaticMesh|AddInstance (Variables|Default|GetRoom) (Math|Transform|MakeTransform (Math|Vector|MakeVector (.X (Math|Vector|BreakVector (+ (+ (Math|Vector|MakeVector (* _index_8 -2e+02) (* _index_2 (* (- (Variables|Default|GetLength) 2) 2e+02)) -1.1e+02) "-310.000000,90.000000,-100.000000") (* "0.000000,20.000000, 0" _index_2)))) (.Y (Math|Vector|BreakVector (+ (+ (Math|Vector|MakeVector (* _index_8 -2e+02) (* _index_2 (* (- (Variables|Default|GetLength) 2) 2e+02)) -1.1e+02) "-310.000000,90.000000,-100.000000") (* "0.000000,20.000000, 0" _index_2)))) (+ (* -1 (LocalVariables|GetHighWallOffset)) -2e+02)) (Math|Rotator|MakeRotator 9e+01 0.0 (* _index_2 1.8e+02)) "1,1,1"))))))))