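; Elevator actor that descends in two stages from top through middle to bottom, then fades out and opens the next level, or the main menu on game over.
; Gameplay messages drive a state machine whose transitions start movement; entering top, middle or bottom snaps the floor into place.
; One timeline moves the floor and spins instanced ropes, played in reverse with negated offset for the second descent, which disables player input.
; Construction builds an instanced 8x8 floor without corners.
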(event Custom|OnTopStateChangeToGoingDownState
  (bind _ropes (Variables|Default|GetRopes))
  (bind _returnvalue (Components|InstancedStaticMesh|GetInstanceCount _ropes))
  (bind _returnvalue_2 (- _returnvalue 1))
  (Variables|Default|SetTargetStateName (Variables|Default|GetMiddleStateName))
  (Components|Activation|Activate (Variables|Default|GetElevatorMovingAudio) false)
  (bind (_direction _elevatorzlocation _roperotationspeed) (Timeline|ElevatorMoving PlayFromStart)
    (:Update
      (Transformation|SetRelativeLocation (Variables|Default|GetFloor) (Math|Vector|MakeVector 0.0 0.0 (* _elevatorzlocation (Variables|Default|GetRelativeOffset))) false true)
      (for _index (range 0 _returnvalue_2)
        (if (.ReturnValue (Components|InstancedStaticMesh|GetInstanceTransform _ropes _index false))
          (Components|InstancedStaticMesh|UpdateInstanceTransform _ropes _index (Math|Transform|MakeTransform (.Location (Math|Transform|BreakTransform (.OutInstanceTransform (Components|InstancedStaticMesh|GetInstanceTransform _ropes _index false)))) (Math|Rotator|CombineRotators (.Rotation (Math|Transform|BreakTransform (.OutInstanceTransform (Components|InstancedStaticMesh|GetInstanceTransform _ropes _index false)))) (Math|Rotator|MakeRotator 0.0 0.0 (* (Utilities|Select :Index _direction :Forward 1 :Backward -1) _roperotationspeed))) (.Scale (Math|Transform|BreakTransform (.OutInstanceTransform (Components|InstancedStaticMesh|GetInstanceTransform _ropes _index false))))) false (select (== _index _returnvalue_2) true false) true))))
    (:Finished
      (Class|GeneralStateMachineComponent|ChangeStateto (Variables|Default|GetGeneralStateMachine) (Variables|Default|GetTargetStateName))
      ;[1 1 1] 判断是否为GameOver，不是的话则进入到下一个关卡。
      (if (Variables|Default|GetReadyToFinish)
        (Class|WorldManager|StartFadewithEvent (Subsystems|GetWorldManager) (EventDispatchers|CreateEvent :!event Custom|OnGameCompleted) false 0.5)))
    (:CollisionSound
      (Components|Activation|Activate (Variables|Default|GetCollisionAudio) false))))

(event Custom|OnGameCompleted
  (bind _returnvalue (Subsystems|GetWorldManager))
  ;[1 1 1] 判断是否为GameOver，不是的话则进入到下一个关卡。
  (if (Variables|Default|GetIsGameOver)
    (Class|WorldManager|OpenNewLevel _returnvalue "MainMenu")
    (else
      (Class|WorldManager|OpenNewLevel _returnvalue (Variables|Default|GetNew%20Level%20ID)))))

(event Custom|OnGetGoingDownMessage
  (params (Message :type GMS%20Message%20Base%20Object%20Reference))
  (Class|GeneralStateMachineComponent|ChangeStateto (Variables|Default|GetGeneralStateMachine) (Variables|Default|GetGoingDownStateName)))

(event Custom|OnGetGoingDownSecondlyMessage
  (params (Message :type GMS%20Message%20Base%20Object%20Reference))
  (Class|GeneralStateMachineComponent|ChangeStateto (Variables|Default|GetGeneralStateMachine) (Variables|Default|GetGoingDownSecondlyStateName)))

(event Custom|OnEnterBottomState
  (Transformation|SetRelativeLocation (Variables|Default|GetFloor) "0, 0,-2100.000000" false true))

(event Custom|OnEnterTopState
  (Transformation|SetRelativeLocation (Variables|Default|GetFloor) "0, 0,2100.000000" false true))

(event Custom|OnMiddleStateChangeToGoingDownSecondlyState
  (bind _returnvalue (Game|GetPlayerController 0))
  (bind _ropes (Variables|Default|GetRopes))
  (bind _returnvalue_2 (Components|InstancedStaticMesh|GetInstanceCount _ropes))
  (bind _returnvalue_3 (- _returnvalue_2 1))
  (Variables|Default|SetTargetStateName (Variables|Default|GetBottomStateName))
  (Components|Activation|Activate (Variables|Default|GetElevatorMovingAudio) false)
  (Input|DisableInput _returnvalue _returnvalue)
  (Variables|Default|SetRelativeOffset -1.0)
  (Variables|Default|SetReadyToFinish true)
  (Class|GameplayMessageSubsystem|Broadcast (Subsystems|GetGameplayMessageSubsystem) "(TagName=\"GMSMessage.Gameplay.DisableKillVolume\")")
  (bind (_direction _elevatorzlocation _roperotationspeed) (Timeline|ElevatorMoving ReverseFromEnd)
    (:Update
      (Transformation|SetRelativeLocation (Variables|Default|GetFloor) (Math|Vector|MakeVector 0.0 0.0 (* _elevatorzlocation (Variables|Default|GetRelativeOffset))) false true)
      (for _index (range 0 _returnvalue_3)
        (if (.ReturnValue (Components|InstancedStaticMesh|GetInstanceTransform _ropes _index false))
          (Components|InstancedStaticMesh|UpdateInstanceTransform _ropes _index (Math|Transform|MakeTransform (.Location (Math|Transform|BreakTransform (.OutInstanceTransform (Components|InstancedStaticMesh|GetInstanceTransform _ropes _index false)))) (Math|Rotator|CombineRotators (.Rotation (Math|Transform|BreakTransform (.OutInstanceTransform (Components|InstancedStaticMesh|GetInstanceTransform _ropes _index false)))) (Math|Rotator|MakeRotator 0.0 0.0 (* (Utilities|Select :Index _direction :Forward 1 :Backward -1) _roperotationspeed))) (.Scale (Math|Transform|BreakTransform (.OutInstanceTransform (Components|InstancedStaticMesh|GetInstanceTransform _ropes _index false))))) false (select (== _index _returnvalue_3) true false) true))))
    (:Finished
      (Class|GeneralStateMachineComponent|ChangeStateto (Variables|Default|GetGeneralStateMachine) (Variables|Default|GetTargetStateName))
      ;[1 1 1] 判断是否为GameOver，不是的话则进入到下一个关卡。
      (if (Variables|Default|GetReadyToFinish)
        (Class|WorldManager|StartFadewithEvent (Subsystems|GetWorldManager) (EventDispatchers|CreateEvent :!event Custom|OnGameCompleted) false 0.5)))
    (:CollisionSound
      (Components|Activation|Activate (Variables|Default|GetCollisionAudio) false))))

(event Custom|OnEnterMiddleState
  (Transformation|SetRelativeLocation (Variables|Default|GetFloor) "0, 0, 0" false true)
  (Default|CallOnEnterMiddleStateDispathcer))

(event EventEndPlay
  (params (EndPlayReason :type EEndPlayReason%20Enum :default "Destroyed"))
  (bind _returnvalue (Subsystems|GetGameplayMessageSubsystem))
  (bind _goingdownsecondlygmshandle (Variables|Default|GetGoingDownSecondlyGMSHandle))
  (bind _goingdowngmshandle (Variables|Default|GetGoingDownGMSHandle))
  (Utilities|FlowControl|Sequence
    (:then_0
      (if (Class|GameplayMessageSubsystem|IsHandleValid _goingdowngmshandle)
        (Class|GameplayMessageSubsystem|Unregister _returnvalue _goingdowngmshandle)))
    (:then_1
      (if (Class|GameplayMessageSubsystem|IsHandleValid _goingdownsecondlygmshandle)
        (Class|GameplayMessageSubsystem|Unregister _returnvalue _goingdownsecondlygmshandle)))))

(event EventBeginPlay
  (bind _returnvalue (Subsystems|GetGameplayMessageSubsystem))
  (bind _generalstatemachine (Variables|Default|GetGeneralStateMachine))
  (Utilities|FlowControl|Sequence
    (:then_1
      (bind _returnvalue_2 (Class|GameplayMessageSubsystem|Register _returnvalue "(TagName=\"GMSMessage.Gameplay.CenterRoom.ElevatorGoingDown\")" (EventDispatchers|CreateEvent :!event Custom|OnGetGoingDownMessage)))
      (Variables|Default|SetGoingDownGMSHandle _returnvalue_2)
      (bind _returnvalue_3 (Class|GameplayMessageSubsystem|Register _returnvalue "(TagName=\"GMSMessage.Gameplay.CenterRoom.ElevatorGoingDownSecondly\")" (EventDispatchers|CreateEvent :!event Custom|OnGetGoingDownSecondlyMessage)))
      (Variables|Default|SetGoingDownSecondlyGMSHandle _returnvalue_3))
    (:then_2
      (Class|GeneralStateMachineComponent|CreateStateMachineNodeBP _generalstatemachine (Variables|Default|GetTopStateName))
      (Class|GeneralStateMachineComponent|CreateStateMachineNodeBP _generalstatemachine (Variables|Default|GetBottomStateName))
      (Class|GeneralStateMachineComponent|CreateStateMachineNodeBP _generalstatemachine (Variables|Default|GetGoingDownStateName))
      (Class|GeneralStateMachineComponent|CreateStateMachineNodeBP _generalstatemachine (Variables|Default|GetGoingDownSecondlyStateName))
      (Class|GeneralStateMachineComponent|CreateStateMachineNodeBP _generalstatemachine (Variables|Default|GetMiddleStateName)))
    (:then_3
      (Class|GeneralStateMachineComponent|SetStateMachineConditionwithAction _generalstatemachine (Variables|Default|GetTopStateName) (Variables|Default|GetGoingDownStateName) (EventDispatchers|CreateEvent :!event Custom|OnTopStateChangeToGoingDownState))
      (Class|GeneralStateMachineComponent|SetStateMachineCondition _generalstatemachine (Variables|Default|GetGoingDownStateName) (Variables|Default|GetMiddleStateName))
      (Class|GeneralStateMachineComponent|SetStateMachineNodeonEnterStateDelegate _generalstatemachine (Variables|Default|GetBottomStateName) (EventDispatchers|CreateEvent :!event Custom|OnEnterBottomState))
      (Class|GeneralStateMachineComponent|SetStateMachineConditionwithAction _generalstatemachine (Variables|Default|GetMiddleStateName) (Variables|Default|GetGoingDownSecondlyStateName) (EventDispatchers|CreateEvent :!event Custom|OnMiddleStateChangeToGoingDownSecondlyState))
      (Class|GeneralStateMachineComponent|SetStateMachineCondition _generalstatemachine (Variables|Default|GetGoingDownSecondlyStateName) (Variables|Default|GetBottomStateName))
      (Class|GeneralStateMachineComponent|SetStateMachineNodeonEnterStateDelegate _generalstatemachine (Variables|Default|GetTopStateName) (EventDispatchers|CreateEvent :!event Custom|OnEnterTopState))
      (Class|GeneralStateMachineComponent|SetStateMachineNodeonEnterStateDelegate _generalstatemachine (Variables|Default|GetMiddleStateName) (EventDispatchers|CreateEvent :!event Custom|OnEnterMiddleState))
      (Class|GeneralStateMachineComponent|InitGeneralStateMachine _generalstatemachine (Variables|Default|GetTopStateName)))))

(fn ConstructionScript
  (CallFunction|CreateFloor)
  (Transformation|SetMobility (Variables|Default|GetChildActor) "Movable"))

(fn CreateFloor
  (for _index (range 0 7)
    (for _index_2 (range 0 7)
      (if (and (or (!= _index 0) (and (!= _index_2 0) (!= _index_2 7))) (or (!= _index 7) (and (!= _index_2 0) (!= _index_2 7))))
        (Components|InstancedStaticMesh|AddInstance (Variables|Default|GetFloor) (Math|Transform|MakeTransform (+ (+ (Math|Vector|MakeVector (* _index_2 2e+02) (* _index 2e+02) 0.0) (LocalVariables|GetOffSet)) (Math|Random|RandomFloatinRange 0.0 0.01)) "0, 0, 0" "1,1,1"))))))