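; Start-room delivery machine actor that opens on a deliver button message and, after the first door opening, supplies an ID card.
; An Idling/Opening state machine plays the open animation forward or in reverse; an empty machine closes itself after a delay.
; The first-door message snaps it shut, spawns the attached card and starts a knocking sound, removed on the next opening.
; Gameplay messages drive it, and taking the card broadcasts the FlashLight message.
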(event Custom|On%20Deliver%20Button%20Pressed
  (params (Message :type GMS%20Message%20Base%20Object%20Reference))
  (bind _generalstatemachine (Variables|Default|GetGeneralStateMachine))
  (if (Class|GeneralStateMachineComponent|IsSameState (Variables|Default|GetGeneralStateMachine) "Idling")
    (Class|GeneralStateMachineComponent|ChangeStateto _generalstatemachine "Opening")
    (Variables|Default|GetIDCard
      (:then
        (EventDispatchers|UnbindEventfromOnAudioFinished (Variables|Default|GetKnockingSoundComponent) (EventDispatchers|CreateEvent :!event Custom|PlayingKnockAudio))
        (CallFunction|OnKnockingAudioFinished))
      (:else
        (Utilities|FlowControl|Delay 3.0)
        (if (not (Variables|Default|GetOnFirstOpeningDoorDeceived))
          (Class|GeneralStateMachineComponent|ChangeStateto _generalstatemachine "Idling"))))))

(event Custom|OnFirstOpenDoorReceived
  (params (Message :type GMS%20Message%20Base%20Object%20Reference))
  (Variables|Default|SetOnFirstOpeningDoorDeceived true)
  (Class|GeneralStateMachineComponent|ChangeStateto (Variables|Default|GetGeneralStateMachine) "Idling")
  (CallFunction|CreateIDCard)
  (Utilities|FlowControl|Delay 0.5)
  (bind _returnvalue (Class|AudioSubsystem|SpawnSound3D (Subsystems|GetAudioSubsystem) "MainLevel_DeliverKnockSound" "0, 0, 0" "0, 0, 0" -1.0 false))
  (bind _output_get (Variables|Default|SetKnockingSoundComponent _returnvalue))
  (Transformation|AttachComponentToComponent _output_get (Variables|Default|GetDeliverMachine) "None" "KeepRelative" "KeepRelative" "KeepRelative" true)
  (EventDispatchers|BindEventtoOnAudioFinished (Variables|Default|GetKnockingSoundComponent) (EventDispatchers|CreateEvent :!event Custom|PlayingKnockAudio)))

(event Custom|OnIDCardBeenTaken
  (params (DestroyedActor :type Actor%20Object%20Reference))
  (Class|GameplayMessageSubsystem|Broadcast (Subsystems|GetGameplayMessageSubsystem) "(TagName=\"GMSMessage.Gameplay.StartRoom.FlashLight\")" 0 false))

(event Custom|CreateIDCard
  (bind _returnvalue (Game|SpawnActorfromClass "/Game/AYR/Blueprints/Interactable/IDCard/BPA_IDCard.BPA_IDCard_C" (Math|Transform|MakeTransform "0, 0, 0" "0, 0, 0" "1,1,1") "Undefined" 0 "NewEnumerator0" 0))
  (bind _output_get (Variables|Default|SetIDCard _returnvalue))
  (Transformation|AttachComponentToComponent _output_get (Variables|Default|GetDeliverMachine) "IDCardLocation" "KeepRelative" "KeepRelative" "KeepWorld" true)
  (Game|BindEventtoOnDestroyed (Variables|Default|GetIDCard) (EventDispatchers|CreateEvent :!event Custom|OnIDCardBeenTaken)))

(event Custom|OnKnockingAudioFinished
  (Components|DestroyComponent (Variables|Default|GetKnockingSoundComponent))
  (Variables|Default|SetKnockingSoundComponent 0))

(event Custom|PlayingKnockAudio
  (bind _knockingsoundcomponent (Variables|Default|GetKnockingSoundComponent))
  (Utilities|FlowControl|Delay (Math|Random|RandomFloatinRange 2.0 6.0))
  (Utilities|IsValid _knockingsoundcomponent
    (:Is%20Valid
      (Audio|Components|Audio|Play _knockingsoundcomponent 0.0))))

(event EventBeginPlay
  (bind _returnvalue (Subsystems|GetGameplayMessageSubsystem))
  (bind _generalstatemachine (Variables|Default|GetGeneralStateMachine))
  (Utilities|FlowControl|Sequence
    (:then_0
      (Class|GeneralStateMachineComponent|CreateStateMachineNode _generalstatemachine "Idling")
      (Class|GeneralStateMachineComponent|CreateStateMachineNode _generalstatemachine "Opening"))
    (:then_1
      (Class|GeneralStateMachineComponent|SetStateMachineConditionwithCheckandAction _generalstatemachine "Idling" "Opening" (EventDispatchers|CreateEvent :!event StateCheck) (EventDispatchers|CreateEvent :!event OnEnterOpeningStateCheckPassed))
      (Class|GeneralStateMachineComponent|SetStateMachineConditionwithCheckandAction _generalstatemachine "Opening" "Idling" (EventDispatchers|CreateEvent :!event StateCheck) (EventDispatchers|CreateEvent :!event OnEnterIdlingStateCheckPassed))
      (Class|GeneralStateMachineComponent|InitGeneralStateMachine _generalstatemachine "Idling"))
    (:then_2
      (bind _returnvalue_2 (Class|GameplayMessageSubsystem|Register _returnvalue "(TagName=\"GMSMessage.Gameplay.StartRoom.DeliverMachine\")" (EventDispatchers|CreateEvent :!event Custom|On%20Deliver%20Button%20Pressed)))
      (Variables|Default|SetGMSHandle _returnvalue_2)
      (bind _returnvalue_3 (Class|GameplayMessageSubsystem|Register _returnvalue "(TagName=\"GMSMessage.Gameplay.StartRoom.FirstOpenDoor\")" (EventDispatchers|CreateEvent :!event Custom|OnFirstOpenDoorReceived)))
      (Variables|Default|SetFirstOpeningDoorGMSHandle _returnvalue_3))))

(event EventEndPlay
  (params (EndPlayReason :type EEndPlayReason%20Enum :default "Destroyed"))
  (bind _returnvalue (Subsystems|GetGameplayMessageSubsystem))
  (Class|GameplayMessageSubsystem|Unregister _returnvalue (Variables|Default|GetGMSHandle))
  (Class|GameplayMessageSubsystem|Unregister _returnvalue (Variables|Default|GetFirstOpeningDoorGMSHandle)))

(fn ConstructionScript
  (Components|Animation|OverrideAnimationData (Variables|Default|GetDeliverMachine) "/Game/AYR/Meshes/DeliverMachine/AS_DeliverMachine_Open.AS_DeliverMachine_Open" false false 0.0 -1.0))

(fn StateCheck
  (return (or (not (Audio|Components|Audio|IsPlaying (Variables|Default|GetDeliverMachine))) (Variables|Default|GetOnFirstOpeningDoorDeceived))))

(fn OnEnterIdlingStateCheckPassed
  (bind _delivermachine (Variables|Default|GetDeliverMachine))
  (if (Variables|Default|GetOnFirstOpeningDoorDeceived)
    (Components|Animation|SetPosition _delivermachine 0.0 true)
    (Audio|Components|Audio|Stop _delivermachine)
    (else
      (Components|Timeline|SetPlayRate _delivermachine -1.0)
      (Audio|Components|Audio|Play _delivermachine false))))

(fn OnEnterOpeningStateCheckPassed
  (bind _delivermachine (Variables|Default|GetDeliverMachine))
  (Components|Timeline|SetPlayRate _delivermachine 1.0)
  (Audio|Components|Audio|Play _delivermachine false))