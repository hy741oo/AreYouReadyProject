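; BPA_Door is a sliding door actor that opens and closes in response to gameplay messages.
; On BeginPlay it makes the door component movable and registers listeners for valid opening and closing tags, unregistering them on EndPlay.
; A timeline drives the door's relative Y location, playing to open and reversing to close.
; Both messages also play a 3D door-moving sound at the actor through the audio subsystem.
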(event Custom|OpenDoor
  (bind _door (Variables|Default|GetDoor))
  (bind _relativelocation (Variables|/Script/Engine.SceneComponent|GetRelativeLocation _door))
  (bind (_x _y _z) (Math|Vector|BreakVector _relativelocation))
  (bind _doorrelativeylocation (Timeline|Timeline_0 Play)
    (:Update
      (Transformation|SetRelativeLocation _door (Math|Vector|MakeVector _x _doorrelativeylocation _z) false false))))

(event Custom|CloseDoor
  (bind _door (Variables|Default|GetDoor))
  (bind _relativelocation (Variables|/Script/Engine.SceneComponent|GetRelativeLocation _door))
  (bind (_x _y _z) (Math|Vector|BreakVector _relativelocation))
  (bind _doorrelativeylocation (Timeline|Timeline_0 Reverse)
    (:Update
      (Transformation|SetRelativeLocation _door (Math|Vector|MakeVector _x _doorrelativeylocation _z) false false))))

(event Custom|OnOpeningDoorMessageReceived
  (params (Message :type GMS%20Message%20Base%20Object%20Reference))
  (bind _returnvalue (Transformation|GetActorTransform))
  (bind (_location _rotation) (Math|Transform|BreakTransform _returnvalue))
  (CallFunction|OpenDoor)
  (Class|AudioSubsystem|PlaySound3D (Subsystems|GetAudioSubsystem) "MainLevel_DoorMoving" _location _rotation -1.0 0))

(event Custom|OnClosingDoorMessageReceived
  (params (Message :type GMS%20Message%20Base%20Object%20Reference))
  (bind _returnvalue (Transformation|GetActorTransform))
  (bind (_location _rotation) (Math|Transform|BreakTransform _returnvalue))
  (CallFunction|CloseDoor)
  (Class|AudioSubsystem|PlaySound3D (Subsystems|GetAudioSubsystem) "MainLevel_DoorMoving" _location _rotation -1.0 0))

(event EventBeginPlay
  (bind _returnvalue (Subsystems|GetGameplayMessageSubsystem))
  (bind _closingopeningdoorgmstag (Variables|GMSTag|GetClosingOpeningDoorGMSTag))
  (bind _openingdoorgmstag (Variables|GMSTag|GetOpeningDoorGMSTag))
  (Utilities|FlowControl|Sequence
    (:then_0
      (if (GameplayTags|IsGameplayTagValid _closingopeningdoorgmstag)
        (bind _returnvalue_2 (Class|GameplayMessageSubsystem|Register _returnvalue _closingopeningdoorgmstag (EventDispatchers|CreateEvent :!event Custom|OnClosingDoorMessageReceived)))
        (Variables|GMSHandle|SetClosingDoorGMSHandle _returnvalue_2)))
    (:then_1
      (if (GameplayTags|IsGameplayTagValid _openingdoorgmstag)
        (bind _returnvalue_3 (Class|GameplayMessageSubsystem|Register _returnvalue _openingdoorgmstag (EventDispatchers|CreateEvent :!event Custom|OnOpeningDoorMessageReceived)))
        (Variables|GMSHandle|SetOpeningDoorGMSHandle _returnvalue_3)))
    (:then_2
      (Transformation|SetMobility (Variables|Default|GetDoor) "Movable"))))

(event EventEndPlay
  (params (EndPlayReason :type EEndPlayReason%20Enum :default "Destroyed"))
  (bind _returnvalue (Subsystems|GetGameplayMessageSubsystem))
  (bind _openingdoorgmshandle (Variables|GMSHandle|GetOpeningDoorGMSHandle))
  (bind _closingdoorgmshandle (Variables|GMSHandle|GetClosingDoorGMSHandle))
  (Utilities|FlowControl|Sequence
    (:then_0
      (if (Class|GameplayMessageSubsystem|IsHandleValid _openingdoorgmshandle)
        (Class|GameplayMessageSubsystem|Unregister _returnvalue _openingdoorgmshandle)))
    (:then_1
      (if (Class|GameplayMessageSubsystem|IsHandleValid _closingdoorgmshandle)
        (Class|GameplayMessageSubsystem|Unregister _returnvalue _closingdoorgmshandle)))))

(fn ConstructionScript)