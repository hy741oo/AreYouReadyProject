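; Corridor actor that builds a modular hallway of configurable length and runs a sequential lights-out effect.
; The construction script tiles instanced floor, ceiling and wall pieces, adds a spotlight per segment and offsets end doorframe walls by the length.
; A gameplay message listener, registered between BeginPlay and EndPlay, drives the delayed recursive shutoff, hiding lights one by one with 3D sound.
; Separate events switch all lights on or off instantly.
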(event Custom|TurnOnLight
  (for _array_element (Variables|Default|GetSpotLight)
    (Rendering|SetVisibility _array_element true false)))

(event Custom|TurnOffLight
  (for _array_element (Variables|Default|GetSpotLight)
    (Rendering|SetVisibility _array_element false false)))

(event Custom|CloseLightOrderly
  (params (Message :type GMS%20Message%20Base%20Object%20Reference))
  (Variables|Default|SetTempSpotLight (Variables|Default|GetSpotLight))
  (Utilities|FlowControl|Delay 0.5)
  (CallFunction|CloseLightRecursivly))

(event Custom|CloseLightRecursivly
  (bind _tempspotlight (Variables|Default|GetTempSpotLight))
  (bind _output (Utilities|Array|Get(acopy) _tempspotlight))
  (if (> (Utilities|Array|Length _tempspotlight) 0)
    (Rendering|SetVisibility _output false false)
    (Class|AudioSubsystem|PlaySound3D (Subsystems|GetAudioSubsystem) "MainLevel_CorridorTurnOffLight" (Transformation|GetWorldLocation _output) "0, 0, 0" -1.0 0)
    (Utilities|Array|RemoveIndex _tempspotlight)
    (Utilities|FlowControl|Delay 0.6)
    (CallFunction|CloseLightRecursivly)))

(event EventBeginPlay
  (bind _corridoreventgmstag (Variables|Default|GetCorridorEventGMSTag))
  (if (GameplayTags|IsGameplayTagValid _corridoreventgmstag)
    (bind _returnvalue (Class|GameplayMessageSubsystem|Register (Subsystems|GetGameplayMessageSubsystem) _corridoreventgmstag (EventDispatchers|CreateEvent :!event Custom|CloseLightOrderly)))
    (Variables|Default|SetCloseLightGMSHandle _returnvalue)))

(event EventEndPlay
  (params (EndPlayReason :type EEndPlayReason%20Enum :default "Destroyed"))
  (bind _closelightgmshandle (Variables|Default|GetCloseLightGMSHandle))
  (if (Class|GameplayMessageSubsystem|IsHandleValid _closelightgmshandle)
    (Class|GameplayMessageSubsystem|Unregister (Subsystems|GetGameplayMessageSubsystem) _closelightgmshandle)))

(fn ConstructionScript
  (CallFunction|CreateCorridor))

(fn CreateCorridor
  (bind _room (Variables|Default|GetRoom))
  (bind _length (Variables|Default|GetLength))
  (bind _room_2 (Variables|Default|GetRoom))
  (bind _room_3 (Variables|Default|GetRoom))
  (bind _returnvalue (* _length 6e+02))
  (bind _returnvalue_2 (+ _returnvalue 2e+01))
  (bind _returnvalue_3 (* _returnvalue_2 -1.0))
  (bind _returnvalue_4 (Math|Vector|MakeVector 0.0 0.0 _returnvalue_3))
  (Components|InstancedStaticMesh|ClearInstances (Variables|Default|GetRoom))
  (Utilities|Array|Clear (Variables|Default|GetSpotLight))
  (for _index (range 0 (- (Variables|Default|GetLength) 1))
    (for _index_2 (range 0 2)
      (LocalVariables|SetOffset (+ (* _index_2 2e+02) (* _index 6e+02)))
      (Utilities|FlowControl|Sequence
        (:then_0
          ;[1 1 1] 地板和天花板。
          (Components|InstancedStaticMesh|AddInstance _room_3 (Math|Transform|MakeTransform (Math|Vector|MakeVector (LocalVariables|GetOffset) 0.0 0.0) "0, 0, 0" "1.000001,1.000001,1.000001"))
          (Components|InstancedStaticMesh|AddInstance _room_3 (Math|Transform|MakeTransform (Math|Vector|MakeVector (LocalVariables|GetOffset) 0.0 4.1e+02) "0, 0,180.000000" "1.000001,1.000001,1.000001")))
        (:then_1
          ;[1 1 1] 左侧墙壁。
          (Components|InstancedStaticMesh|AddInstance _room (Math|Transform|MakeTransform (Math|Vector|MakeVector (LocalVariables|GetOffset) -1.1e+02 1.1e+02) "0, 0,90.000000" "1.000001,1.000001,1.000001"))
          (Components|InstancedStaticMesh|AddInstance _room (Math|Transform|MakeTransform (Math|Vector|MakeVector (LocalVariables|GetOffset) -1.1e+02 3.1e+02) "0, 0,90.000000" "1.000001,1.000001,1.000001")))
        (:then_2
          ;[1 1 1] 左侧墙壁。
          (Components|InstancedStaticMesh|AddInstance _room_2 (Math|Transform|MakeTransform (Math|Vector|MakeVector (LocalVariables|GetOffset) 1.1e+02 1.1e+02) "0, 0,-90.000000" "1.000001,1.000001,1.000001"))
          (Components|InstancedStaticMesh|AddInstance _room_2 (Math|Transform|MakeTransform (Math|Vector|MakeVector (LocalVariables|GetOffset) 1.1e+02 3.1e+02) "0, 0,-90.000000" "1.000001,1.000001,1.000001")))
        (:then_3
          ;[1 1 1] 添加吸顶灯。
          (if (== _index_2 1)
            (bind _returnvalue_5 (AddComponent|AddSpotLightComponent false (Math|Transform|MakeTransform (Math|Vector|MakeVector (LocalVariables|GetOffset) 0.0 3.9e+02) "-90.000000, 0, 0" "1.000001,1.000001,1.000001")))
            (Utilities|Array|Add (Variables|Default|GetSpotLight) _returnvalue_5))))))
  (Transformation|AddLocalOffset (Variables|Default|GetRoomWallWithDoorframeEndLocation) _returnvalue_4 false true)
  (Transformation|AddLocalOffset (Variables|Default|GetRoomWallWithExtraDoorframeEndLocation) _returnvalue_4 false true))